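; BP_AfterImage is a self-destroying ghost actor that shows a frozen afterimage of a skeletal mesh's pose.
; Event_InitFromMesh copies the source pose onto the PMGhost poseable mesh and applies a dynamic AfterImageMaterial to its first material slot.
; The TL_Fade timeline lerps Opacity from StartOpacity to EndOpacity, then destroys the actor.
; The Tint and initial Opacity setters are disconnected, so Tint is never applied.
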(event Custom|Event_InitFromMesh
  (params (SourceMesh :type Skeletal%20Mesh%20Component%20Object%20Reference))
  (bind _pm_ghost (Variables|Default|GetPM_Ghost))
  (Utilities|IsValid SourceMesh
    (:Is%20Valid
      (Class|PoseableMeshComponent|CopyPosefromSkeletalComponent _pm_ghost SourceMesh)
      (bind _returnvalue (Rendering|Material|CreateDynamicMaterialInstance _pm_ghost 0 (Variables|Default|GetAfterImageMaterial) "None" :!class /Script/Engine.PrimitiveComponent))
      (bind _output_get (Variables|Default|SetMID _returnvalue))
      (bind _alpha (Timeline|TL_Fade PlayFromStart)
        (:Update
          (Rendering|Material|SetScalarParameterValue (Variables|Default|GetMID) "Opacity" (Math|Float|Lerp (Variables|Default|GetStartOpacity) (Variables|Default|GetEndOpacity) _alpha) :!class /Script/Engine.MaterialInstanceDynamic))
        (:Finished
          (Actor|DestroyActor))))))

(event EventBeginPlay)

(event Collision|EventActorBeginOverlap
  (params (OtherActor :type Actor%20Object%20Reference)))

(event EventTick
  (params (DeltaSeconds :type Float%20%28single-precision%29)))

(fn ConstructionScript)