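; BP_AfterImage_Weapon is a short-lived afterimage actor that leaves a fading ghost copy of a weapon.
; Event_InitFromWeaponActor copies the mesh and world transform of the weapon's first static mesh component onto SMWeaponGhost, then applies a dynamic M_AfterImage material to slot 0.
; A timeline lerps the material's Opacity from start to end value and destroys the actor when finished.
; The Tint and initial Opacity setters are unconnected and never run.
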(event Custom|Event_InitFromWeaponActor
  (params (WeaponActor :type BP%20Weapon%20Object%20Reference))
  (bind _returnvalue (Actor|GetComponentsByClass WeaponActor "/Script/Engine.StaticMeshComponent"))
  (bind _sm_weaponghost (Variables|Default|GetSM_WeaponGhost))
  (bind _output (Utilities|Array|Get(acopy) _returnvalue))
  (Utilities|IsValid WeaponActor
    (:Is%20Valid
      (Utilities|IsValid _output
        (:Is%20Valid
          (Components|StaticMesh|SetStaticMesh _sm_weaponghost (Variables|/Script/Engine.StaticMeshComponent|GetStaticMesh _output))
          (Transformation|SetWorldTransform _sm_weaponghost (Transformation|GetWorldTransform _output) false false)
          (bind _returnvalue_2 (Rendering|Material|CreateDynamicMaterialInstance _sm_weaponghost 0 "/Game/_Core/FX/M_AfterImage.M_AfterImage" "None" :!class /Script/Engine.PrimitiveComponent))
          (bind _output_get (Variables|Default|SetMID _returnvalue_2))
          (bind _alpha (Timeline|TL_Fade PlayFromStart)
            (:Update
              (Rendering|Material|SetScalarParameterValue (Variables|Default|GetMID) "Opacity" (Math|Float|Lerp (Variables|Default|GetStartOpacity) (Variables|Default|GetEndOpacity) _alpha) :!class /Script/Engine.MaterialInstanceDynamic))
            (:Finished
              (Actor|DestroyActor))))))))

(event EventBeginPlay)

(event Collision|EventActorBeginOverlap
  (params (OtherActor :type Actor%20Object%20Reference)))

(event EventTick
  (params (DeltaSeconds :type Float%20%28single-precision%29)))

(fn ConstructionScript)