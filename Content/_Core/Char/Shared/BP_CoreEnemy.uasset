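; BP_CoreEnemy is a base enemy character that provides a shared attack animation and floating damage numbers.
; PlayMonsterAttack plays the AttackMontage assigned in child Blueprints, skipping the call if that montage is already playing.
; BeginPlay caches HP and binds to the Health change event, which spawns a BP_DamageFloaterActor above the capsule showing the truncated HP loss.
; The cached HP updates only on damage, so healing leaves it unchanged.
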(event Custom|Event_OnHealthChanged
  (params (NewHP :type Float%20%28single-precision%29) (MaxHP :type Float%20%28single-precision%29))
  (bind _output_get (Variables|Default|SetDamage (- (Variables|Default|GetPrevHP) NewHP)))
  (if (> _output_get 0.0)
    (bind _returnvalue (Game|SpawnActorfromClass "/Game/_Core/UI/Combat/BP_DamageFloaterActor.BP_DamageFloaterActor_C" (Math|Transform|MakeTransform (+ (Transformation|GetActorLocation) (Math|Vector|MakeVector 0.0 0.0 (+ (Components|Capsule|GetScaledCapsuleHalfHeight (Variables|Default|GetCapsuleComponent)) 5e+01))) "0, 0, 0" "1.000000,1.000000,1.000000") "Undefined" "MultiplyWithRoot" 0 0))
    (Default|Init _returnvalue (Math|Float|Truncate (Variables|Default|GetDamage)))
    (Variables|Default|SetPrevHP NewHP)))

(event EventBeginPlay
  (bind _health (Variables|Default|GetHealth))
  (Variables|Default|SetPrevHP (Class|HealthComponent|GetHP _health))
  (EventDispatchers|BindEventtoOnHealthChanged _health (delegate Custom|Event_OnHealthChanged)))

(event Collision|EventActorBeginOverlap
  (params (OtherActor :type Actor%20Object%20Reference)))

(event EventTick
  (params (DeltaSeconds :type Float%20%28single-precision%29)))

(event EventPlayMonsterAttack
  (bind _mesh (Variables|Character|GetMesh))
  ;[0.15 0.15 0.15 0.5] 자식 BP의 디테일에서 AttackMontage검색에서 할당하면 됨
  (if (not (Animation|Montage|MontageIsPlaying (Components|SkeletalMesh|GetAnimInstance _mesh) (Variables|Default|GetAttackMontage)))
    (Animation|Montage|PlayMontage _mesh (Variables|Default|GetAttackMontage))))

(fn ConstructionScript)