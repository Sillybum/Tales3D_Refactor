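; Shared core character Blueprint that handles combat animation, effects and HP/combo widgets, and grants Cassandra's rapier on BeginPlay.
; Health and Combo component events update the widgets, showing the combo only from two hits.
; Plays five-section basic combo montages; skill playback always uses AM_Skill1, and non-combo montage endings notify Skills and Combo when a skill is active.
; Skill data drives Niagara effects and mesh/weapon afterimages.
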(event Custom|Event_OnComboChanged
  (params (NewCount :type Integer))
  ;[0.15 0.15 0.15 0.5] 콤보카운트UI 초기화 & 델리게이트 이벤트 연결
  (if (< NewCount 2)
    (Rendering|SetVisibility (Variables|Default|GetWC_Combo) false false)
    (Default|EventUpdateCombo (Variables|Default|GetComboWidgetRef) NewCount)
    (else
      (Rendering|SetVisibility (Variables|Default|GetWC_Combo) true false)
      (Utilities|IsValid (Variables|Default|GetComboWidgetRef)
        (:Is%20Valid
          (Default|EventUpdateCombo (Variables|Default|GetComboWidgetRef) NewCount))))))

(event Custom|Event_OnHPChanged
  (params (NewHP :type Float%20%28single-precision%29) (MaxHP :type Float%20%28single-precision%29))
  (bind _hpwidgetref (Variables|Default|GetHPWidgetRef))
  (Utilities|IsValid _hpwidgetref
    (:Is%20Valid
      (Default|UpdateHP _hpwidgetref NewHP MaxHP))))

(event Custom|OnMontageEnded_Event
  (params (Montage :type Anim%20Montage%20Object%20Reference) (bInterrupted :type Boolean))
  (bind _skills (Variables|Default|GetSkills))
  (if (not (== Montage "/Game/_Core/Char/Shared/Anim/Montage/AM_BasicCombo.AM_BasicCombo"))
    (if (Class|SkillComponent|IsSkillActive _skills)
      (Class|SkillComponent|NotifyActiveSkillEnded _skills)
      (Class|ComboComponent|NotifySkillMontageEnded (Variables|Default|GetCombo)))))

(event EventPlaySkillMontage
  (params (Montage :type Anim%20Montage%20Object%20Reference))
  (bind _mesh (Variables|Character|GetMesh))
  (bind _returnvalue (Components|SkeletalMesh|GetAnimInstance _mesh))
  ;[0.15 0.15 0.15 0.5] Play Skill1 Montage
  (Utilities|IsValid Montage
    (:Is%20Valid
      (Animation|Montage|MontageStop _returnvalue 0.05 "/Game/_Core/Char/Shared/Anim/Montage/AM_BasicCombo.AM_BasicCombo")
      (Animation|Montage|MontagePlay _returnvalue "/Game/_Core/Char/Shared/Anim/Montage/AM_Skill1.AM_Skill1" 1.0 "MontageLength" 0.0 true))))

(event EventBeginPlay
  (bind _wc_combo (Variables|Default|GetWC_Combo))
  (bind _health (Variables|Default|GetHealth))
  (|CallParentFunction)
  (EventDispatchers|AssignOnMontageEnded (Components|SkeletalMesh|GetAnimInstance (Variables|Character|GetMesh)) (delegate Custom|OnMontageEnded_Event))
  (Class|InventoryComponent|AddItemData (Variables|Default|GetInventory) "/Game/_Core/Data/Item/DA_Rapier_Cassandra.DA_Rapier_Cassandra" 1)
  ;[0.15 0.15 0.15 0.5] 콤보카운트UI 초기화 & 델리게이트 이벤트 연결
  (bind _aswbp_combo (Utilities|Casting|CastToWBP_Combo (UserInterface|GetUserWidgetObject _wc_combo)))
  (Variables|Default|SetComboWidgetRef _aswbp_combo)
  (Rendering|SetVisibility _wc_combo false false)
  (EventDispatchers|BindEventtoOnComboCountChanged (Variables|Default|GetCombo) (delegate Custom|Event_OnComboChanged))
  ;[0.15 0.15 0.15 0.5] HP 초기화
  (bind _aswbp_hpbar (Utilities|Casting|CastToWBP_HPBar (UserInterface|GetUserWidgetObject (Variables|Default|GetWC_PlayerHP))))
  (bind _output_get (Variables|Default|SetHPWidgetRef _aswbp_hpbar))
  (Default|UpdateHP _output_get (Class|HealthComponent|GetHP _health) (Class|HealthComponent|GetMaxHP _health))
  (EventDispatchers|BindEventtoOnHealthChanged (Variables|Default|GetHealth) (delegate Custom|Event_OnHPChanged)))

(event EventSpawnSkillEffectFX
  (params (SkillData :type Core%20Skill%20Data%20Object%20Reference) (TargetActor :type Actor%20Object%20Reference))
  ;[0.15 0.15 0.15 0.5] Effect FX
  (Utilities|FlowControl|Sequence
    (:then_0
      (Variables|Default|SetEffectFXSkillData SkillData)
      (Variables|Default|SetEffectFXTargetActor TargetActor))
    (:then_1
      (Utilities|IsValid (Variables|Default|GetEffectFXSkillData)
        (:Is%20Valid
          (Utilities|IsValid (Variables|/Script/Tales3D_Refactor.CoreSkillData|GetEffectFX (Variables|Default|GetEffectFXSkillData))
            (:Is%20Valid
              (if (Variables|/Script/Tales3D_Refactor.CoreSkillData|GetbAttachEffectFXToOwner (Variables|Default|GetEffectFXSkillData))
                (Niagara|SpawnSystemAttached (Variables|/Script/Tales3D_Refactor.CoreSkillData|GetEffectFX (Variables|Default|GetEffectFXSkillData)) (Variables|Character|GetMesh) (Variables|/Script/Tales3D_Refactor.CoreSkillData|GetEffectFXSocket (Variables|Default|GetEffectFXSkillData)) "0, 0, 0" "0, 0, 0" "SnapToTarget" true)
                (else
                  (Utilities|IsValid (Variables|Default|GetEffectFXTargetActor)
                    (:Is%20Valid
                      (if (Variables|/Script/Tales3D_Refactor.CoreSkillData|GetbSpawnEffectFXAtTarget (Variables|Default|GetEffectFXSkillData))
                        (Niagara|SpawnSystematLocation (Variables|/Script/Tales3D_Refactor.CoreSkillData|GetEffectFX (Variables|Default|GetEffectFXSkillData)) (Transformation|GetActorLocation (Variables|Default|GetEffectFXTargetActor)))
                        (else
                          (Niagara|SpawnSystematLocation (Variables|/Script/Tales3D_Refactor.CoreSkillData|GetEffectFX (Variables|Default|GetEffectFXSkillData)) (+ (Transformation|GetActorLocation (Variables|Default|GetEffectFXTargetActor)) (* (Transformation|GetActorForwardVector (Variables|Default|GetEffectFXTargetActor)) 1e+02))))))))))))))))

(event EventSpawnSkillAfterImageFX
  (params (SkillData :type Core%20Skill%20Data%20Object%20Reference))
  (bind _mesh (Variables|Character|GetMesh))
  (bind _mesh_2 (Variables|Character|GetMesh))
  (bind _returnvalue (Transformation|GetWorldTransform _mesh))
  (bind _output_get (Variables|Default|SetAfterImageSkillData SkillData))
  (Utilities|IsValid _output_get
    (:Is%20Valid
      (if (Variables|/Script/Tales3D_Refactor.CoreSkillData|GetbUseAfterImage (Variables|Default|GetAfterImageSkillData))
        (if (Utilities|IsValidClass (Variables|/Script/Tales3D_Refactor.CoreSkillData|GetAfterImageActorClass (Variables|Default|GetAfterImageSkillData)))
          (bind _returnvalue_2 (Game|SpawnActorfromClass (Variables|/Script/Tales3D_Refactor.CoreSkillData|GetAfterImageActorClass (Variables|Default|GetAfterImageSkillData)) _returnvalue "Undefined" "MultiplyWithRoot" 0 0))
          (bind _asbp_after_image (Utilities|Casting|CastToBP_AfterImage _returnvalue_2))
          (Default|EventInitfromMesh _asbp_after_image _mesh_2)
          (else
            (bind _returnvalue_3 (Game|SpawnActorfromClass "/Game/_Core/FX/BP_AfterImage.BP_AfterImage_C" _returnvalue "Undefined" "MultiplyWithRoot" 0 0))
            (Default|EventInitfromMesh _returnvalue_3 _mesh_2)))
        (bind _array_element (Utilities|Array|ForEachLoopwithBreak (Actor|GetAttachedActors true false) :!label _label)
          (:LoopBody
            (if (Actor|ActorHasTag _array_element "EquippedWeapon")
              (bind _output_get_2 (Variables|Default|SetWeaponActor _array_element))
              (goto _label Break)))
          (:Completed
            (Utilities|IsValid _output_get_2
              (:Is%20Valid
                (bind _returnvalue_4 (Game|SpawnActorfromClass "/Game/_Core/FX/BP_AfterImage_Weapon.BP_AfterImage_Weapon_C" (Transformation|GetActorTransform _output_get_2) "Undefined" "MultiplyWithRoot" 0 0))
                (bind _asbp_weapon (Utilities|Casting|CastToBP_Weapon _output_get_2))
                (Default|EventInitfromWeaponActor _returnvalue_4 _asbp_weapon)))))))))

(event EventPlayBasicAttackSection
  (params (SectionIndex :type Integer))
  (bind _mesh (Variables|Character|GetMesh))
  (bind _returnvalue (Components|SkeletalMesh|GetAnimInstance _mesh))
  (Utilities|IsValid _returnvalue
    (:Is%20Valid
      (if (Animation|Montage|MontageIsPlaying _returnvalue "/Game/_Core/Char/Shared/Anim/Montage/AM_BasicCombo.AM_BasicCombo")
        _
        (else
          (Animation|Montage|MontagePlay _returnvalue "/Game/_Core/Char/Shared/Anim/Montage/AM_BasicCombo.AM_BasicCombo" 1.0 "MontageLength" 0.0 true)))
      (Ability|Animation|MontageJumptoSection _returnvalue (Utilities|Select :Index (- (Math|Integer|Clamp(Integer) SectionIndex 1 5) 1) :Option%200 "A1" :Option%201 "A2" :Option%202 "A3" :Option%203 "A4" :Option%204 "A5") "/Game/_Core/Char/Shared/Anim/Montage/AM_BasicCombo.AM_BasicCombo"))))

(fn ConstructionScript)